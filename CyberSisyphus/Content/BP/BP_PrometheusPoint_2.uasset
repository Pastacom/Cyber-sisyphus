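; Prometheus Point actor that swaps a delivered BP_Boulder for a BP_HalvedBoulder through a timed mechanical sequence.
; One box registers the boulder; the player then leaving Box1 triggers a delayed, one-time sequence.
; Chained timelines rotate StaticMesh3 and lower the GD53MOD1A2AndreCoelho component 400 units.
; It then reveals BoulderHalf, destroys the boulder, spawns the halved one at the actor, and raises the component while rotating the mesh back.
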(event `self.ReceiveBeginPlay`
  (bind _returnvalue (`SceneComponent.K2_GetComponentLocation` (`self.GD53_MOD1_A2_AndreCoelho`)))
  (set `self.HighPosition` _returnvalue)
  (set `self.LowPosition` (+ _returnvalue (0.0 0.0 -400.0))))

(event `self.Box.OnComponentBeginOverlap`
  (params (OverlappedComponent :type "PrimitiveComponent Object Reference") (OtherActor :type "Actor Object Reference") (OtherComp :type "PrimitiveComponent Object Reference") (OtherBodyIndex :type Integer) (bFromSweep :type Boolean) (SweepResult :type "HitResult Structure (by ref)"))
  (bind _asbp_boulder (cast `/Game/BP/BP_Boulder` OtherActor))
  (set `self.As BP Boulder` _asbp_boulder)
  (set `self.BoulderIn` true))

(event `self.Box1.OnComponentEndOverlap`
  (params (OverlappedComponent :type "PrimitiveComponent Object Reference") (OtherActor :type "Actor Object Reference") (OtherComp :type "PrimitiveComponent Object Reference") (OtherBodyIndex :type Integer))
  (cast `/Game/TopDown/Blueprints/BP_TopDownCharacter` OtherActor)
  (if (`self.BoulderIn`)
    (`/Engine/EditorBlueprintResources/StandardMacros.DoOnce` false
      (:`Completed`
        (`KismetSystemLibrary.Delay` 3.0)
        (bind (_direction _newtrack_1) (`Timeline|Timeline`)
          (:`Update`
            (`SceneComponent.K2_SetRelativeRotation` (`self.StaticMesh3`) (`KismetMathLibrary.RLerp` (struct :`Pitch` -90.0) (struct) _newtrack_1) false false))
          (:`Finished`
            (bind (_direction_2 _newtrack_1_2) (`Timeline|Timeline_0`)
              (:`Update`
                (`SceneComponent.K2_SetWorldLocation` (`self.GD53_MOD1_A2_AndreCoelho`) (`KismetMathLibrary.VLerp` (`self.HighPosition`) (`self.LowPosition`) _newtrack_1_2) false false))
              (:`Finished`
                (`KismetSystemLibrary.Delay` 1.0)
                (`SceneComponent.SetHiddenInGame` (`self.BoulderHalf`) false false)
                (`self.K2_DestroyActor` (`self.As BP Boulder`))
                (bind _returnvalue (`|SpawnActorFromClass` "/Game/BP/BP_HalvedBoulder.BP_HalvedBoulder_C" (`KismetMathLibrary.Conv_VectorToTransform` (`KismetMathLibrary.Vector_Zero`)) "Undefined" "MultiplyWithRoot" null null))
                (`SceneComponent.K2_SetWorldLocation` (`Actor.RootComponent` _returnvalue) (`self.K2_GetActorLocation`) false false)
                (bind (_direction_3 _newtrack_1_3) (`Timeline|Timeline_1`)
                  (:`Update`
                    (`SceneComponent.K2_SetWorldLocation` (`self.GD53_MOD1_A2_AndreCoelho`) (`KismetMathLibrary.VLerp` (`self.LowPosition`) (`self.HighPosition`) _newtrack_1_3) false false)
                    (bind (_direction_4 _newtrack_1_4) (`Timeline|Timeline_2`)
                      (:`Update`
                        (`SceneComponent.K2_SetRelativeRotation` (`self.StaticMesh3`) (`KismetMathLibrary.RLerp` (struct) (struct :`Pitch` -90.0) _newtrack_1_4) false false)))))))))))))

(fn `UserConstructionScript`)