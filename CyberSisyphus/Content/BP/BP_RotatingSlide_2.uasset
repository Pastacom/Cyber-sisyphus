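; BP_RotatingSlide_2 is a powered mechanism that the player rotates while interacting with it.
; An activation point reference toggles its Powered state, and events bound on BP_TopDownCharacter start and stop the motion.
; A fast looping timer applies small local rotations, unpausing only when powered with the interaction button held, and pausing on the stop event.
; A MoveDoor helper lerps a mesh between two angles but is not called here.
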(event `self.ReceiveBeginPlay`
  (bind _returnvalue (`GameplayStatics.GetActorOfClass` "/Game/TopDown/Blueprints/BP_TopDownCharacter.BP_TopDownCharacter_C"))
  (set `self.Player` _returnvalue)
  (add `/Game/BP/BP_ActivationPoint.Activate` (`self.ActivationPointRef`) (delegate `PowerUpMechanism`))
  (add `/Game/TopDown/Blueprints/BP_TopDownCharacter.Activate2` (`self.Player`) (delegate `ActivateMechanism`))
  (bind _returnvalue_2 (`KismetSystemLibrary.K2_SetTimerDelegate` (delegate `CustomEvent`) 0.0005 true))
  (bind _output_get (set `self.TimerHandle` _returnvalue_2))
  (`KismetSystemLibrary.K2_PauseTimerHandle` _output_get)
  (add `/Game/TopDown/Blueprints/BP_TopDownCharacter.Stop` (`self.Player`) (delegate `CustomEvent_1`)))

(event `CustomEvent_1`
  (`KismetSystemLibrary.K2_PauseTimerHandle` (stale `self.ReceiveBeginPlay` _output_get)))

(event `PowerUpMechanism`
  (set `self.Powered` (not (`self.Powered`))))

(event `CustomEvent`
  (`self.K2_AddActorLocalRotation` (struct :`Yaw` 0.01)))

(event `ActivateMechanism`
  (if (and (`/Game/TopDown/Blueprints/BP_TopDownCharacter.IsMechanismInteractionButtonHeld` (`self.Player`)) (`self.Powered`))
    (`KismetSystemLibrary.K2_UnPauseTimerHandle` (`self.TimerHandle`))))

(fn `Move Door`
  (params (Alpha :type "Float (double-precision)") (DoorMesh :type "StaticMeshComponent Object Reference"))
  (`SceneComponent.K2_SetRelativeRotation` DoorMesh (`KismetMathLibrary.RLerp` (`self.StartAngle`) (`self.EndAngle`) Alpha true) false false))

(fn `UserConstructionScript`)