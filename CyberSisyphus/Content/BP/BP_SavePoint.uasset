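; Save point actor that autosaves the game when the top-down character enters its box trigger.
; A DoOnce fires on the first overlap by any actor, then casts to the character.
; It saves player and boulder transforms offset from its own transform, plus the character's pulse cannon and projector flags, to the "autosave" slot.
; A save widget appears before saving and is removed after a short delay.
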(event `self.Box.OnComponentBeginOverlap`
  (params (OverlappedComponent :type "PrimitiveComponent Object Reference") (OtherActor :type "Actor Object Reference") (OtherComp :type "PrimitiveComponent Object Reference") (OtherBodyIndex :type Integer) (bFromSweep :type Boolean) (SweepResult :type "HitResult Structure (by ref)"))
  (bind (_returnvalue_location _returnvalue_rotation) (`KismetMathLibrary.BreakTransform` (`self.GetTransform`)))
  (`/Engine/EditorBlueprintResources/StandardMacros.DoOnce` false
    (:`Completed`
      (bind _asbp_top_down_character (cast `/Game/TopDown/Blueprints/BP_TopDownCharacter` OtherActor))
      (bind _returnvalue (`|CreateWidget` "/Game/UI/SaveWidget.SaveWidget_C" (`GameplayStatics.GetPlayerController` 0)))
      (bind _output_get (set `self.SaveWidget` _returnvalue))
      (`UserWidget.AddToViewport` _output_get 0)
      (bind _returnvalue_2 (`GameplayStatics.CreateSaveGameObject` "/Game/BP/BP_SaveGame.BP_SaveGame_C"))
      (set `/Game/BP/BP_SaveGame.PlayerPosition` (`KismetMathLibrary.MakeTransform` (+ _returnvalue_location (0.0 0.0 50.0)) _returnvalue_rotation) _returnvalue_2)
      (set `/Game/BP/BP_SaveGame.BoulderPosition` (`KismetMathLibrary.MakeTransform` (+ _returnvalue_location (100.0 100.0 100.0)) _returnvalue_rotation) _returnvalue_2)
      (set `/Game/BP/BP_SaveGame.IsPulseCanonInstalled` (`/Game/TopDown/Blueprints/BP_TopDownCharacter.IsPulseCanonInstalled` _asbp_top_down_character) _returnvalue_2)
      (set `/Game/BP/BP_SaveGame.IsProjectorInstalled` (`/Game/TopDown/Blueprints/BP_TopDownCharacter.IsProjectorInstalled` _asbp_top_down_character) _returnvalue_2)
      (`GameplayStatics.SaveGameToSlot` _returnvalue_2 "autosave")
      (`KismetSystemLibrary.Delay` 2.0)
      (`Widget.RemoveFromParent` (`self.SaveWidget`)))))

(fn `UserConstructionScript`)