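; BP_HalvedBoulder is a boulder actor that the player interacts with to trigger a core installation.
; On BeginPlay it finds BP_TopDownCharacter and binds PressButtonEvent to that character's interact event.
; When pressed while the player overlaps the Sphere component, it hides a second sphere component and calls InstallCore on the character.
; The overlap is checked only on press, and nothing here prevents repeat triggering.
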(event `self.ReceiveBeginPlay`
  (bind _returnvalue (`GameplayStatics.GetActorOfClass` "/Game/TopDown/Blueprints/BP_TopDownCharacter.BP_TopDownCharacter_C"))
  (bind _output_get (set `self.Player` _returnvalue))
  (add `/Game/TopDown/Blueprints/BP_TopDownCharacter.Interact` _output_get (delegate `PressButtonEvent`)))

(event `PressButtonEvent`
  (if (`PrimitiveComponent.IsOverlappingActor` (`self.Sphere`) (`self.Player`))
    (`SceneComponent.SetHiddenInGame` (`self.Sphere_3FAA5286`) true false)
    (`/Game/TopDown/Blueprints/BP_TopDownCharacter.InstallCore` (`self.Player`))))

(fn `UserConstructionScript`)