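; BP_PulseCannon is a top-down player cannon that turns with the mouse cursor and fires pulse explosions.
; On BeginPlay it caches the controller and character and binds Fire to a character event.
; Tick yaws Turret4 along the flattened cursor-to-ShotPoint direction.
; Fire drains player energy, then, if the cursor hits something, traces from ShotPoint toward it and spawns BP_PulseExplosion at the trace's hit location.
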(event `self.ReceiveBeginPlay`
  (bind _returnvalue (`GameplayStatics.GetActorOfClass` "/Game/TopDown/Blueprints/BP_TopDownController.BP_TopDownController_C"))
  (set `self.TopDownController` _returnvalue)
  (bind _returnvalue_2 (`GameplayStatics.GetActorOfClass` "/Game/TopDown/Blueprints/BP_TopDownCharacter.BP_TopDownCharacter_C"))
  (set `self.Player` _returnvalue_2)
  (add `/Game/TopDown/Blueprints/BP_TopDownCharacter.Fire` _returnvalue_2 (delegate `Fire`)))

(event `Fire`
  (bind (_hit _location) (`self.GetLocationUnderCursor`))
  (`/Game/TopDown/Blueprints/BP_TopDownCharacter.DecreaseEnergy` (`self.Player`) 1.0)
  (if _hit
    (bind _outhit (`KismetSystemLibrary.LineTraceSingle` (`SceneComponent.K2_GetComponentLocation` (`self.ShotPoint`)) _location "TraceTypeQuery1" false (`|MakeArray` (`self.Player`) :!type "Actor Object Reference")))
    (`|SpawnActorFromClass` "/Game/BP/BP_PulseExplosion.BP_PulseExplosion_C" (`KismetMathLibrary.Conv_VectorToTransform` (`.Location` (`GameplayStatics.BreakHitResult` _outhit))) "Undefined" "MultiplyWithRoot" null null)))

(event `self.ReceiveTick`
  (params (DeltaSeconds :type "Float (single-precision)"))
  (bind _returnvalue (`KismetMathLibrary.GetDirectionUnitVector` (`.Location` (`self.GetLocationUnderCursor`)) (`SceneComponent.K2_GetComponentLocation` (`self.ShotPoint`))))
  (`SceneComponent.K2_SetWorldRotation` (`self.turret4`) (`KismetMathLibrary.Conv_VectorToRotator` (+ (* _returnvalue (`KismetMathLibrary.Vector_Forward`)) (* _returnvalue (`KismetMathLibrary.Vector_Right`)))) false false))

(fn `GetAngle`
  (params (A :type "Vector Structure") (B :type "Vector Structure"))
  (returns (NewParam :type "Float (double-precision)"))
  (return (`KismetMathLibrary.DegAcos` (`KismetMathLibrary.Dot_VectorVector` A B))))

(fn `GetLocationUnderCursor`
  (returns (Hit :type Boolean) (Location :type "Vector Structure"))
  (bind (_bblockinghit _binitialoverlap _time _distance _location) (`GameplayStatics.BreakHitResult` (`PlayerController.GetHitResultUnderCursorByChannel` (`self.TopDownController`) "TraceTypeQuery1" true)))
  (return _bblockinghit _location))

(fn `UserConstructionScript`)