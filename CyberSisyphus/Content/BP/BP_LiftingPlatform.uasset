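; Lifting platform that rises along its up vector while powered and while the player holds the mechanism interaction button.
; At BeginPlay it binds to a referenced activation point, which toggles power, and to the top-down character's activation event.
; That event plays a slowed Timeline that lerps the cube toward a fixed offset, rechecking both conditions each update and stopping in place when either fails.
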(event `self.ReceiveBeginPlay`
  (bind _returnvalue (`SceneComponent.K2_GetComponentLocation` (`self.DefaultSceneRoot`)))
  (bind _returnvalue_2 (`GameplayStatics.GetActorOfClass` "/Game/TopDown/Blueprints/BP_TopDownCharacter.BP_TopDownCharacter_C"))
  (set `self.Player` _returnvalue_2)
  (`TimelineComponent.SetPlayRate` (`self.Timeline_0`) 0.3)
  (add `/Game/BP/BP_ActivationPoint.Activate` (`self.ActivationPointRef`) (delegate `PowerUpMechanism`))
  (add `/Game/TopDown/Blueprints/BP_TopDownCharacter.Activate2` (`self.Player`) (delegate `ActivateMechanism`))
  (set `self.StartPosition` _returnvalue)
  (set `self.EndPosition` (+ _returnvalue (* (`self.GetActorUpVector`) (500.0 500.0 500.0)))))

(event `PowerUpMechanism`
  (set `self.Powered` (not (`self.Powered`))))

(event `ActivateMechanism`
  (if (and (`/Game/TopDown/Blueprints/BP_TopDownCharacter.IsMechanismInteractionButtonHeld` (`self.Player`)) (`self.Powered`)) :!label _label
    (bind (_direction _newtrack_0) (`Timeline|Timeline_0`)
      (:`Update`
        (`SceneComponent.K2_SetWorldLocation` (`self.Cube`) (`KismetMathLibrary.VLerp` (`self.StartPosition`) (`self.EndPosition`) _newtrack_0) false false)
        (goto _label)))
    (else
      (`TimelineComponent.Stop` (`self.Timeline_0`)))))

(fn `UserConstructionScript`)