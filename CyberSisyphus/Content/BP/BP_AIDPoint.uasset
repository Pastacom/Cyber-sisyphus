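; BP_AIDPoint is a trigger point that starts a one-time scripted sequence involving the boulder and the player.
; A boulder entering Box sets a flag, which arms the player's exit from Box1.
; That exit rotates StaticMesh3 by timeline after a delay, then spawns BP_Manipulator_2 high above the point.
; After another delay it plays the AID sound and drains player energy through an endless Delay loop.
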(event `self.Box.OnComponentBeginOverlap`
  (params (OverlappedComponent :type "PrimitiveComponent Object Reference") (OtherActor :type "Actor Object Reference") (OtherComp :type "PrimitiveComponent Object Reference") (OtherBodyIndex :type Integer) (bFromSweep :type Boolean) (SweepResult :type "HitResult Structure (by ref)"))
  (cast `/Game/BP/BP_Boulder` OtherActor)
  (set `self.BoulderIn` true))

(event `self.Box1.OnComponentEndOverlap`
  (params (OverlappedComponent :type "PrimitiveComponent Object Reference") (OtherActor :type "Actor Object Reference") (OtherComp :type "PrimitiveComponent Object Reference") (OtherBodyIndex :type Integer))
  (cast `/Game/TopDown/Blueprints/BP_TopDownCharacter` OtherActor)
  (if (`self.BoulderIn`)
    (`/Engine/EditorBlueprintResources/StandardMacros.DoOnce` false
      (:`Completed`
        (`KismetSystemLibrary.Delay` 3.0)
        (bind (_direction _newtrack_1) (`Timeline|Timeline`)
          (:`Update`
            (`SceneComponent.K2_SetRelativeRotation` (`self.StaticMesh3`) (`KismetMathLibrary.RLerp` (struct :`Pitch` -90.0) (struct) _newtrack_1) false false))
          (:`Finished`
            (`|SpawnActorFromClass` "/Game/StarterBundle/Manipulator/source/BP_Manipulator_2.BP_Manipulator_2_C" (`KismetMathLibrary.MakeTransform` (+ (`self.K2_GetActorLocation`) (0.0 500.0 2500.0)) (struct :`Roll` -125.0)) "Undefined" "MultiplyWithRoot" null null)
            (`KismetSystemLibrary.Delay` 4.0)
            (`GameplayStatics.PlaySound2D` "/Game/Sounds/WAV_AID.WAV_AID" 0.6 1.0 0.0 null null)
            (bind _asbp_top_down_character (cast `/Game/TopDown/Blueprints/BP_TopDownCharacter` (`GameplayStatics.GetPlayerCharacter` 0)))
            (`/Game/TopDown/Blueprints/BP_TopDownCharacter.DecreaseEnergy` _asbp_top_down_character 0.7 :!label _label)
            (`KismetSystemLibrary.Delay` 0.1)
            (goto _label)))))))

(fn `UserConstructionScript`)