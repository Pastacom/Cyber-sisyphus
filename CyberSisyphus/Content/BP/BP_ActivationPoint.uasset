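; BP_ActivationPoint is a pressure-plate-style trigger that responds to a BP_Boulder entering or leaving its box.
; Boulder overlaps brighten or dim the top-down character's Movecontraption UI element.
; When the boulder's Collider enters, it fires the Activate dispatcher, turns the cylinder blue and plays a sound.
; When that Collider exits, it fires Activate again, turns the cylinder red, stops the sound and fires Deactivate.
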(event `self.Box.OnComponentBeginOverlap`
  (params (OverlappedComponent :type "PrimitiveComponent Object Reference") (OtherActor :type "Actor Object Reference") (OtherComp :type "PrimitiveComponent Object Reference") (OtherBodyIndex :type Integer) (bFromSweep :type Boolean) (SweepResult :type "HitResult Structure (by ref)"))
  (bind _asbp_boulder (cast `/Game/BP/BP_Boulder` OtherActor))
  (bind _returnvalue (`GameplayStatics.GetActorOfClass` "/Game/TopDown/Blueprints/BP_TopDownCharacter.BP_TopDownCharacter_C"))
  (set `Widget.RenderOpacity` 1.0 (`/Game/UI/UI.Movecontraption` (`/Game/TopDown/Blueprints/BP_TopDownCharacter.UI` _returnvalue)))
  (if (== OtherComp (`/Game/BP/BP_Boulder.Collider` _asbp_boulder))
    (`self.Activate`)
    (`PrimitiveComponent.SetMaterial` (`self.Cylinder`) 0 "/Game/LevelPrototyping/Materials/MI_Solid_Blue.MI_Solid_Blue")
    (bind _returnvalue_2 (`GameplayStatics.SpawnSound2D` "/Game/StarterContent/Audio/Light01.Light01" 0.2 1.0 0.0 null))
    (set `self.Sound` _returnvalue_2)))

(event `self.Box.OnComponentEndOverlap`
  (params (OverlappedComponent :type "PrimitiveComponent Object Reference") (OtherActor :type "Actor Object Reference") (OtherComp :type "PrimitiveComponent Object Reference") (OtherBodyIndex :type Integer))
  (bind _asbp_boulder (cast `/Game/BP/BP_Boulder` OtherActor))
  (bind _returnvalue (`GameplayStatics.GetActorOfClass` "/Game/TopDown/Blueprints/BP_TopDownCharacter.BP_TopDownCharacter_C"))
  (set `Widget.RenderOpacity` 0.5 (`/Game/UI/UI.Movecontraption` (`/Game/TopDown/Blueprints/BP_TopDownCharacter.UI` _returnvalue)))
  (if (== OtherComp (`/Game/BP/BP_Boulder.Collider` _asbp_boulder))
    (`self.Activate`)
    (`PrimitiveComponent.SetMaterial` (`self.Cylinder`) 0 "/Game/LevelPrototyping/Materials/MI_Solid_Red.MI_Solid_Red")
    (`AudioComponent.Stop` (`self.Sound`))
    (`self.Deactivate`)))

(fn `UserConstructionScript`)