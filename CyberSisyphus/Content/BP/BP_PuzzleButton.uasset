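; BP_PuzzleButton is an interactable button that broadcasts an OpenDoor event when the player presses it.
; On BeginPlay it binds to the Interact dispatcher of the BP_TopDownCharacter it finds in the level.
; An interaction only fires OpenDoor while that character overlaps the button's Sphere.
; Sphere overlaps toggle the TextRender for any actor and brighten or dim the character's Interact UI prompt.
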(event `self.ReceiveBeginPlay`
  (bind _returnvalue (`GameplayStatics.GetActorOfClass` "/Game/TopDown/Blueprints/BP_TopDownCharacter.BP_TopDownCharacter_C"))
  (set `self.TopDownCharacter` _returnvalue)
  (add `/Game/TopDown/Blueprints/BP_TopDownCharacter.Interact` (`self.TopDownCharacter`) (delegate `PressButtonEvent`)))

(event `PressButtonEvent`
  (if (`PrimitiveComponent.IsOverlappingActor` (`self.Sphere`) (`self.TopDownCharacter`))
    (`self.OpenDoor`)))

(event `self.Sphere.OnComponentBeginOverlap`
  (params (OverlappedComponent :type "PrimitiveComponent Object Reference") (OtherActor :type "Actor Object Reference") (OtherComp :type "PrimitiveComponent Object Reference") (OtherBodyIndex :type Integer) (bFromSweep :type Boolean) (SweepResult :type "HitResult Structure (by ref)"))
  (`SceneComponent.SetVisibility` (`self.TextRender`) true false)
  (bind _asbp_top_down_character (cast `/Game/TopDown/Blueprints/BP_TopDownCharacter` OtherActor))
  (`Widget.SetRenderOpacity` (`/Game/UI/UI.Interact` (`/Game/TopDown/Blueprints/BP_TopDownCharacter.UI` _asbp_top_down_character)) 1.0))

(event `self.Sphere.OnComponentEndOverlap`
  (params (OverlappedComponent :type "PrimitiveComponent Object Reference") (OtherActor :type "Actor Object Reference") (OtherComp :type "PrimitiveComponent Object Reference") (OtherBodyIndex :type Integer))
  (`SceneComponent.SetVisibility` (`self.TextRender`) false false)
  (bind _asbp_top_down_character (cast `/Game/TopDown/Blueprints/BP_TopDownCharacter` OtherActor))
  (`Widget.SetRenderOpacity` (`/Game/UI/UI.Interact` (`/Game/TopDown/Blueprints/BP_TopDownCharacter.UI` _asbp_top_down_character)) 0.5))

(fn `UserConstructionScript`)