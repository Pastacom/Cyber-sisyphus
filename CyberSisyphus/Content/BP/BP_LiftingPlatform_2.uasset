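; Lifting platform that raises its Cube along the actor's up vector while powered and the player holds the mechanism interaction button.
; A child activation point toggles power, and the player's activation event starts a slow timeline that lerps the Cube upward.
; Each update rechecks both conditions, stopping the lift when either fails.
; Deactivation plays a second timeline from the current position back to the start, then resets the lift timeline.
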(event `Return`
  (`TimelineComponent.Stop` (`self.Timeline_0`))
  (`TimelineComponent.SetPlayRate` (`self.Timeline`) 1.0)
  (set `self.LastPosition` (`SceneComponent.K2_GetComponentLocation` (`self.Cube`)))
  (bind (_direction _newtrack_0) (`Timeline|Timeline`)
    (:`Update`
      (`SceneComponent.K2_SetWorldLocation` (`self.Cube`) (`KismetMathLibrary.VLerp` (`self.StartPosition`) (`self.LastPosition`) _newtrack_0) false false))
    (:`Finished`
      (`TimelineComponent.SetNewTime` (`self.Timeline_0`) 0.0))))

(event `self.ReceiveBeginPlay`
  (bind _returnvalue (`SceneComponent.K2_GetComponentLocation` (`self.Cube`)))
  (bind _asbp_activation_point (cast `/Game/BP/BP_ActivationPoint` (`ChildActorComponent.ChildActor` (`self.BP_ActivationPoint`))))
  (set `self.ActivationPointRef` _asbp_activation_point)
  (bind _returnvalue_2 (`GameplayStatics.GetActorOfClass` "/Game/TopDown/Blueprints/BP_TopDownCharacter.BP_TopDownCharacter_C"))
  (set `self.Player` _returnvalue_2)
  (`TimelineComponent.SetPlayRate` (`self.Timeline_0`) 0.07)
  (add `/Game/BP/BP_ActivationPoint.Activate` (`self.ActivationPointRef`) (delegate `PowerUpMechanism`))
  (add `/Game/TopDown/Blueprints/BP_TopDownCharacter.Activate2` (`self.Player`) (delegate `ActivateMechanism`))
  (add `/Game/BP/BP_ActivationPoint.Deactivate` (`self.ActivationPointRef`) (delegate `Return`))
  (set `self.StartPosition` _returnvalue)
  (set `self.EndPosition` (+ _returnvalue (* (`self.GetActorUpVector`) (800.0 800.0 800.0)))))

(event `PowerUpMechanism`
  (set `self.Powered` (not (`self.Powered`))))

(event `ActivateMechanism`
  (if (and (`/Game/TopDown/Blueprints/BP_TopDownCharacter.IsMechanismInteractionButtonHeld` (`self.Player`)) (`self.Powered`)) :!label _label
    (bind (_direction _newtrack_0) (`Timeline|Timeline_0`)
      (:`Update`
        (`SceneComponent.K2_SetWorldLocation` (`self.Cube`) (`KismetMathLibrary.VLerp` (`self.StartPosition`) (`self.EndPosition`) _newtrack_0) false false)
        (goto _label)))
    (else
      (`TimelineComponent.Stop` (`self.Timeline_0`)))))

(fn `UserConstructionScript`)