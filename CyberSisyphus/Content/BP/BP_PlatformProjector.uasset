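; Turret actor that projects a temporary platform toward the cursor when the player's place-platform event fires, costing player energy.
; Tick flattens the cursor-to-ShotPoint direction to the horizontal plane, using it to rotate the turret and offset spawns.
; Fire traces from ShotPoint to the cursor, ignoring player and boulder, and spawns a platform offset back from the hit.
; Only one platform persists: each new one replaces the last, and hitting the existing one removes it.
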(event `self.ReceiveBeginPlay`
  (bind _returnvalue (`GameplayStatics.GetActorOfClass` "/Game/BP/BP_Boulder.BP_Boulder_C"))
  (set `self.Boulder` _returnvalue)
  (bind _returnvalue_2 (`GameplayStatics.GetActorOfClass` "/Game/TopDown/Blueprints/BP_TopDownController.BP_TopDownController_C"))
  (set `self.TopDownController` _returnvalue_2)
  (bind _returnvalue_3 (`GameplayStatics.GetActorOfClass` "/Game/TopDown/Blueprints/BP_TopDownCharacter.BP_TopDownCharacter_C"))
  (bind _output_get (set `self.Player` _returnvalue_3))
  (add `/Game/TopDown/Blueprints/BP_TopDownCharacter.PlacePlatform` _output_get (delegate `Fire`)))

(event `Fire`
  (bind (_hit _location) (`self.GetLocationUnderCursor`))
  (bind _lastplacedplatform (`self.LastPlacedPlatform`))
  (`/Game/TopDown/Blueprints/BP_TopDownCharacter.DecreaseEnergy` (`self.Player`) 1.0)
  (if _hit
    (bind _outhit (`KismetSystemLibrary.LineTraceSingle` (`SceneComponent.K2_GetComponentLocation` (`self.ShotPoint`)) _location "TraceTypeQuery1" false (`|MakeArray` (`self.Player`) (`self.Boulder`) :!type "Actor Object Reference")))
    (bind (_bblockinghit _binitialoverlap _time _distance _location_2 _impactpoint _normal _impactnormal _physmat _hitactor) (`GameplayStatics.BreakHitResult` _outhit))
    (if (== _hitactor _lastplacedplatform)
      (`self.K2_DestroyActor` _lastplacedplatform)
      (else
        (bind _returnvalue (`|SpawnActorFromClass` "/Game/BP/BP_ProjectedPlatform.BP_ProjectedPlatform_C" (`KismetMathLibrary.Conv_VectorToTransform` (+ _location_2 (* (`self.AngleVector`) (200.0 200.0 0.0)))) "Undefined" "MultiplyWithRoot" null null))
        (`self.K2_DestroyActor` (`self.LastPlacedPlatform`))
        (set `self.LastPlacedPlatform` _returnvalue)))))

(event `self.ReceiveTick`
  (params (DeltaSeconds :type "Float (single-precision)"))
  (bind _returnvalue (`KismetMathLibrary.GetDirectionUnitVector` (`.Location` (`self.GetLocationUnderCursor`)) (`SceneComponent.K2_GetComponentLocation` (`self.ShotPoint`))))
  (bind _returnvalue_2 (+ (* _returnvalue (`KismetMathLibrary.Vector_Forward`)) (* _returnvalue (`KismetMathLibrary.Vector_Right`))))
  (set `self.AngleVector` _returnvalue_2)
  (`SceneComponent.K2_SetWorldRotation` (`self.turret4`) (`KismetMathLibrary.Conv_VectorToRotator` _returnvalue_2) false false))

(fn `GetAngle`
  (params (A :type "Vector Structure") (B :type "Vector Structure"))
  (returns (NewParam :type "Float (double-precision)"))
  (return (`KismetMathLibrary.DegAcos` (`KismetMathLibrary.Dot_VectorVector` A B))))

(fn `GetLocationUnderCursor`
  (returns (Hit :type Boolean) (Location :type "Vector Structure"))
  (bind (_bblockinghit _binitialoverlap _time _distance _location) (`GameplayStatics.BreakHitResult` (`PlayerController.GetHitResultUnderCursorByChannel` (`self.TopDownController`) "TraceTypeQuery1" true)))
  (return _bblockinghit _location))

(fn `UserConstructionScript`)