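; A sliding double puzzle door that moves when any of its referenced puzzle buttons fires its open-door event.
; BeginPlay binds OpenDoorEvent to each button and caches both panels' relative start locations and end locations offset in opposite directions along X.
; OpenDoorTimeline lerps the panels between these locations, then swaps start and end so each later trigger reverses the motion.
; A DoOnce gate ignores triggers until the timeline finishes.
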(event `self.ReceiveBeginPlay`
  (bind _returnvalue_location (`KismetMathLibrary.BreakTransform` (`SceneComponent.GetRelativeTransform` (`self.RightDoor`))))
  (bind _returnvalue_location_2 (`KismetMathLibrary.BreakTransform` (`SceneComponent.GetRelativeTransform` (`self.LeftDoor`))))
  (for _array_element (`self.PuzzleButtonRef`)
    (add `/Game/BP/BP_PuzzleButton.OpenDoor` _array_element (delegate `OpenDoorEvent`))
    (set `self.LeftDoorStartLocation` _returnvalue_location_2)
    (set `self.LeftDoorEndLocation` (+ _returnvalue_location_2 (-200.0 0.0 0.0)))
    (set `self.RightDoorStartLocation` _returnvalue_location)
    (set `self.RightDoorEndLocation` (+ _returnvalue_location (200.0 0.0 0.0)))))

(event `OpenDoorEvent`
  (`/Engine/EditorBlueprintResources/StandardMacros.DoOnce` false :!label _label
    (:`Completed`
      (bind (_direction _doorfloat) (`Timeline|OpenDoorTimeline` :!via `PlayFromStart`)
        (:`Update`
          (`SceneComponent.K2_SetRelativeLocation` (`self.LeftDoor`) (`KismetMathLibrary.VLerp` (`self.LeftDoorStartLocation`) (`self.LeftDoorEndLocation`) _doorfloat) false false)
          (`SceneComponent.K2_SetRelativeLocation` (`self.RightDoor`) (`KismetMathLibrary.VLerp` (`self.RightDoorStartLocation`) (`self.RightDoorEndLocation`) _doorfloat) false false))
        (:`Finished`
          (set `self.TempLeft` (`self.LeftDoorStartLocation`))
          (set `self.LeftDoorStartLocation` (`self.LeftDoorEndLocation`))
          (set `self.LeftDoorEndLocation` (`self.TempLeft`))
          (set `self.TempRight` (`self.RightDoorStartLocation`))
          (set `self.RightDoorStartLocation` (`self.RightDoorEndLocation`))
          (set `self.RightDoorEndLocation` (`self.TempRight`))
          (goto _label :!via `Reset`))))))

(fn `UserConstructionScript`)