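; BP_Capsule is a sci-fi capsule actor that travels vertically like an elevator through two custom events.
; MoveDown waits briefly, then lowers the capsule by a fixed offset, while UseElevator raises it immediately by a larger one.
; Each event stores the current location and plays its own Timeline to lerp the actor to the offset position without sweep.
; Nothing in this Blueprint calls either event.
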(event `MoveDown`
  (`KismetSystemLibrary.Delay` 0.5)
  (set `self.Start` (`self.K2_GetActorLocation`))
  (bind (_direction _newtrack_0) (`Timeline|Timeline`)
    (:`Update`
      (`self.K2_SetActorLocation` (`KismetMathLibrary.VLerp` (`self.Start`) (- (`self.Start`) (0.0 0.0 750.0)) _newtrack_0)))))

(event `UseElevator`
  (set `self.Start` (`self.K2_GetActorLocation`))
  (bind (_direction _newtrack_0) (`Timeline|Timeline_0`)
    (:`Update`
      (`self.K2_SetActorLocation` (`KismetMathLibrary.VLerp` (`self.Start`) (+ (`self.Start`) (0.0 0.0 1000.0)) _newtrack_0)))))

(fn `UserConstructionScript`)