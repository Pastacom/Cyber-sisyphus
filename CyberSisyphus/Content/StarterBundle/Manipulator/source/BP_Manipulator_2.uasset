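; BP_Manipulator_2 is an actor that fakes picking up and carrying away the level's BP_Boulder.
; On BeginPlay it stops the boulder's physics and a timeline lerps the manipulator to a fixed offset from the boulder's sphere.
; It then destroys the boulder and unhides its own Sphere in its place.
; A second timeline lerps it back to its start position, where it destroys itself.
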(event `self.ReceiveBeginPlay`
  (set `self.Start` (`self.K2_GetActorLocation`))
  (bind _returnvalue (`GameplayStatics.GetActorOfClass` "/Game/BP/BP_Boulder.BP_Boulder_C"))
  (bind _sphere (`/Game/BP/BP_Boulder.Sphere` _returnvalue))
  (`PrimitiveComponent.SetSimulatePhysics` _sphere false)
  (bind (_direction _newtrack_0) (`Timeline|Timeline`)
    (:`Update`
      (`self.K2_SetActorLocation` (`KismetMathLibrary.VLerp` (`self.Start`) (+ (`SceneComponent.K2_GetComponentLocation` _sphere) (0.0 485.0 1820.0)) _newtrack_0)))
    (:`Finished`
      (`self.K2_DestroyActor` _returnvalue)
      (`SceneComponent.SetHiddenInGame` (`self.Sphere`) false false)
      (set `self.End` (`self.K2_GetActorLocation`))
      (bind (_direction_2 _newtrack_1) (`Timeline|Timeline_0`)
        (:`Update`
          (`self.K2_SetActorLocation` (`KismetMathLibrary.VLerp` (`self.End`) (`self.Start`) _newtrack_1)))
        (:`Finished`
          (`self.K2_DestroyActor`))))))

(fn `UserConstructionScript`)